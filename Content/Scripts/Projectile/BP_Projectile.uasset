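; BP_Projectile is a projectile actor that damages BP_Enemy actors on hit and expires after a short lifespan set at BeginPlay.
; On Hit, it casts the other actor to BP_Enemy, flags it as hit and subtracts the enemy's own DamageTaken from its Health.
; It destroys enemies left without health, then itself.
; Hits on other actors fail the cast, leaving the projectile alive until its lifespan ends.
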(event EventBeginPlay
  (Actor|SetLifeSpan 2.0))

(event Collision|EventActorBeginOverlap
  (params (OtherActor :type Actor%20Object%20Reference)))

(event EventTick
  (params (DeltaSeconds :type Float%20%28single-precision%29)))

(event Collision|EventHit
  (params (MyComp :type Primitive%20Component%20Object%20Reference) (Other :type Actor%20Object%20Reference) (OtherComp :type Primitive%20Component%20Object%20Reference) (bSelfMoved :type Boolean) (HitLocation :type Vector :default "0, 0, 0") (HitNormal :type Vector :default "0, 0, 0") (NormalImpulse :type Vector :default "0, 0, 0") (Hit :type Hit%20Result%20Structure%20%28by%20ref%29))
  (Utilities|IsValid Other
    (:Is%20Valid
      (bind _asbp_enemy (Utilities|Casting|CastToBP_Enemy Other))
      (Variables|/Game/Scripts/Enemy/BP_Enemy.BP_Enemy_C|SetgetHit _asbp_enemy true)
      (bind _output_get (Variables|/Game/Scripts/Enemy/BP_Enemy.BP_Enemy_C|Sethealth _asbp_enemy (- (Variables|/Game/Scripts/Enemy/BP_Enemy.BP_Enemy_C|Gethealth _asbp_enemy) (Variables|/Game/Scripts/Enemy/BP_Enemy.BP_Enemy_C|GetdamageTaken _asbp_enemy))))
      (if (<= _output_get 0)
        (Default|Destroy _asbp_enemy))
      (Actor|DestroyActor))))

(fn ConstructionScript)