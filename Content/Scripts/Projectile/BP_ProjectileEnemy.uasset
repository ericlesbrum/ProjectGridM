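; Enemy projectile Blueprint that damages the player on impact.
; On BeginPlay it caches the player character as a BP_Player reference and gives itself a short lifespan.
; On Hit it calls DamageTaken on that player with a fixed amount and destroys itself, but only when the hit actor is that player.
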(event EventBeginPlay
  (bind _asbp_player (Utilities|Casting|CastToBP_Player (Game|GetPlayerCharacter 0)))
  (Utilities|IsValid _asbp_player
    (:Is%20Valid
      (Variables|Default|SetPlayerRef _asbp_player)
      (Actor|SetLifeSpan 2.0))))

(event Collision|EventActorBeginOverlap
  (params (OtherActor :type Actor%20Object%20Reference)))

(event EventTick
  (params (DeltaSeconds :type Float%20%28single-precision%29)))

(event Collision|EventHit
  (params (MyComp :type Primitive%20Component%20Object%20Reference) (Other :type Actor%20Object%20Reference) (OtherComp :type Primitive%20Component%20Object%20Reference) (bSelfMoved :type Boolean) (HitLocation :type Vector :default "0, 0, 0") (HitNormal :type Vector :default "0, 0, 0") (NormalImpulse :type Vector :default "0, 0, 0") (Hit :type Hit%20Result%20Structure%20%28by%20ref%29))
  (bind _playerref (Variables|Default|GetPlayerRef))
  (Utilities|IsValid Other
    (:Is%20Valid
      (if (== Other _playerref)
        (Default|DamageTaken _playerref 50)
        (Actor|DestroyActor)))))

(fn ConstructionScript)