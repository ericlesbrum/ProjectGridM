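; BP_Gun is an automatic gun that spawns BP_Projectile actors while its trigger is active.
; It caches the player character as BP_Player on BeginPlay and uses that player's Direction component transform as each projectile's spawn transform.
; ActiveTrigger fires immediately, then repeats Fire on a looping timer derived from ShootRate in shots per second.
; DesactiveTrigger clears that timer to stop firing.
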(event Custom|ActiveTrigger
  ;[1 1 1] Fire
  (CallFunction|Fire)
  (Utilities|Time|SetTimerbyFunctionName 0 "Fire" (/ 1.0 (Variables|Default|GetshootRate)) true))

(event Custom|DesactiveTrigger
  ;[1 1 1] Fire
  (Utilities|Time|ClearTimerbyFunctionName 0 "Fire"))

(event EventBeginPlay
  (bind _asbp_player (Utilities|Casting|CastToBP_Player (Game|GetPlayerCharacter 0)))
  (Variables|Default|SetPlayer _asbp_player))

(event Collision|EventActorBeginOverlap
  (params (OtherActor :type Actor%20Object%20Reference)))

(event EventTick
  (params (DeltaSeconds :type Float%20%28single-precision%29)))

(fn ConstructionScript)

(fn Fire
  (Game|SpawnActorfromClass "/Game/Scripts/Projectile/BP_Projectile.BP_Projectile_C" (Transformation|GetWorldTransform (Variables|/Game/Scripts/Player/BP_Player.BP_Player_C|GetDirection (Variables|Default|GetPlayer))) "Undefined" "MultiplyWithRoot" 0 0))