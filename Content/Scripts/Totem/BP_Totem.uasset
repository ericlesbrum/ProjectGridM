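; BP_Totem is an interactable totem that spawns a colored key once the player holds the matching green, pink or blue pickup.
; Interact checks the pickup flag on BP_GameplayGM by TotemType, starts the timeline meant to raise TotemAro, boosts the totem's glow and spawns BP_KeyStatic at the arrow.
; Dynamic material instances set the totem's color and emissive at construction and tint both frames of each spawned key.
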(event EventBeginPlay
  (bind _asbp_gameplay_gm (Utilities|Casting|CastToBP_GameplayGM (Game|GetGameMode)))
  (Variables|Default|SetAs%20BP%20Gameplay%20GM _asbp_gameplay_gm))

(event Collision|EventActorBeginOverlap
  (params (OtherActor :type Actor%20Object%20Reference)))

(event EventInteract
  (bind _as_bp_gameplay_gm (Variables|Default|GetAs%20BP%20Gameplay%20GM))
  (bind _arotimeline (Variables|Default|GetAroTimeLine))
  (switch Utilities|FlowControl|Switch|SwitchonEBP_Keys (Variables|Default|GetTotemType)
    (:NewEnumerator0
      (if (Variables|/Game/Scripts/GameMode/BP_GameplayGM.BP_GameplayGM_C|GetpickUpGreen _as_bp_gameplay_gm)
        (Components|Timeline|PlayfromStart _arotimeline)
        (bind _returnvalue (CallFunction|SpawnKey))
        (CallFunction|ChangeKeyColor _returnvalue "(R=0.000000,G=1.000000,B=0.196078,A=1.000000)")))
    (:NewEnumerator1
      (if (Variables|/Game/Scripts/GameMode/BP_GameplayGM.BP_GameplayGM_C|GetpickUpPink _as_bp_gameplay_gm)
        (Components|Timeline|PlayfromStart _arotimeline)
        (bind _returnvalue_2 (CallFunction|SpawnKey))
        (CallFunction|ChangeKeyColor _returnvalue_2 "(R=1.000000,G=0.000000,B=0.576471,A=1.000000)")))
    (:NewEnumerator2
      (if (Variables|/Game/Scripts/GameMode/BP_GameplayGM.BP_GameplayGM_C|GetpickUpBlue _as_bp_gameplay_gm)
        (Components|Timeline|PlayfromStart _arotimeline)
        (bind _returnvalue_3 (CallFunction|SpawnKey))
        (CallFunction|ChangeKeyColor _returnvalue_3 "(R=0.000000,G=0.200000,B=1.000000,A=1.000000)")))))

(event EventTick
  (params (DeltaSeconds :type Float%20%28single-precision%29)))

(fn ConstructionScript
  (bind _returnvalue (Rendering|Material|CreateDynamicMaterialInstance (Variables|Default|GetTotemBase) 1 "/Game/Models/Totem/M_totemglow.M_totemglow" "None" :!class /Script/Engine.PrimitiveComponent))
  (bind _output_get (Variables|Default|SetTotemMaterial _returnvalue))
  (Rendering|Material|SetScalarParameterValue _output_get "Emissive" (Variables|Default|GetEmissive) :!class /Script/Engine.MaterialInstanceDynamic)
  (Rendering|Material|SetVectorParameterValue _output_get "BaseColor" (Variables|Default|GetColor) :!class /Script/Engine.MaterialInstanceDynamic))

(fn SpawnKey
  (Rendering|Material|SetScalarParameterValue (Variables|Default|GetTotemMaterial) "Emissive" 2e+01 :!class /Script/Engine.MaterialInstanceDynamic)
  (bind _returnvalue (Game|SpawnActorfromClass "/Game/Scripts/Key/BP_KeyStatic.BP_KeyStatic_C" (Transformation|GetWorldTransform (Variables|Default|GetArrow)) "Undefined" "MultiplyWithRoot" 0 0))
  (return _returnvalue))

(fn ChangeKeyColor
  (params (self2 :type BP%20Key%20Static%20Object%20Reference) (KeyColor :type Linear%20Color%20Structure))
  (bind _returnvalue (Rendering|Material|CreateDynamicMaterialInstance (Variables|/Game/Scripts/Key/BP_KeyStatic.BP_KeyStatic_C|Getframe1 self2) 1 "/Game/Models/Key/M_keyglow.M_keyglow" "None" :!class /Script/Engine.PrimitiveComponent))
  (Rendering|Material|SetVectorParameterValue _returnvalue "Param" KeyColor :!class /Script/Engine.MaterialInstanceDynamic)
  (bind _returnvalue_2 (Rendering|Material|CreateDynamicMaterialInstance (Variables|/Game/Scripts/Key/BP_KeyStatic.BP_KeyStatic_C|Getframe2 self2) 1 "/Game/Models/Key/M_keyglow.M_keyglow" "None" :!class /Script/Engine.PrimitiveComponent))
  (Rendering|Material|SetVectorParameterValue _returnvalue_2 "Param" KeyColor :!class /Script/Engine.MaterialInstanceDynamic))