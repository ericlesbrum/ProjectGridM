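; BP_Enemy is a stationary shooting enemy that turns toward the player and fires projectiles.
; An overlap sphere or GetHit flag triggers facing, and a DoOnce starts a looping Fire timer that spawns BP_ProjectileEnemy at the Arrow.
; Separate events stop firing, re-arm the DoOnce and reset detection and health.
; BeginPlay caches the player and randomizes a vertical bobbing range, but the timeline update that would apply it never runs.
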(event OnComponentBeginOverlap(Sphere)
  (params (OverlappedComponent :type Primitive%20Component%20Object%20Reference) (OtherActor :type Actor%20Object%20Reference) (OtherComp :type Primitive%20Component%20Object%20Reference) (OtherBodyIndex :type Integer) (bFromSweep :type Boolean) (SweepResult :type Hit%20Result%20Structure%20%28by%20ref%29))
  (Variables|Default|SetisPlayerOnSight true))

(event OnComponentEndOverlap(Sphere)
  (params (OverlappedComponent :type Primitive%20Component%20Object%20Reference) (OtherActor :type Actor%20Object%20Reference) (OtherComp :type Primitive%20Component%20Object%20Reference) (OtherBodyIndex :type Integer))
  (Variables|Default|SetisPlayerOnSight false))

(event Custom|StopEnemy
  (Utilities|Time|ClearTimerbyFunctionName 0 "Fire"))

(event Custom|RestartEnemy
  (Utilities|FlowControl|DoOnce false) ; enters at Reset
)

(event Custom|ResetStatus
  (Variables|Default|SetisPlayerOnSight false)
  (Variables|Default|SetgetHit false)
  (Variables|Default|Sethealth 100))

(event EventBeginPlay
  (CallFunction|SetonBegin))

(event EventTick
  (params (DeltaSeconds :type Float%20%28single-precision%29))
  (bind _playerref (Variables|Default|GetPlayerRef))
  (if (not (Variables|/Game/Scripts/Player/BP_Player.BP_Player_C|GetisDead _playerref))
    (if (or (Variables|Default|GetisPlayerOnSight) (Variables|Default|GetgetHit))
      (Utilities|FlowControl|Sequence
        (:then_0
          (Transformation|SetActorRotation (Math|Rotator|FindLookatRotation (Transformation|GetActorLocation) (Transformation|GetActorLocation _playerref))))
        (:then_1
          (Utilities|FlowControl|DoOnce false
            (:Completed
              (Utilities|Time|SetTimerbyFunctionName 0 "Fire" (/ 1.0 (Variables|Default|GetshootPerSecond)) true))))))))

(fn ConstructionScript)

(fn SetPosition
  (params (Alpha :type Float%20%28single-precision%29))
  (Transformation|SetActorLocation (Math|Vector|Lerp(Vector) (Variables|Default|GetstartLocation) (Variables|Default|GetendLocation) Alpha) false false))

(fn Fire
  (Game|SpawnActorfromClass "/Game/Scripts/Projectile/BP_ProjectileEnemy.BP_ProjectileEnemy_C" (Transformation|GetWorldTransform (Variables|Default|GetArrow)) "Undefined" "MultiplyWithRoot" 0 0))

(fn SetonBegin
  (Utilities|FlowControl|Sequence
    (:then_0
      (bind _output_get (Variables|Default|SetstartLocation (Transformation|GetActorLocation)))
      (Variables|Default|SetendLocation (+ _output_get (Math|Vector|MakeVector 0.0 0.0 (Math|Random|RandomFloatinRange 5e+01 1e+02))))
      (Components|Timeline|SetPlayRate (Variables|Default|GetEnemy_Loop) (Math|Random|RandomFloatinRange 1.0 2.0)))
    (:then_1
      (bind _asbp_player (Utilities|Casting|CastToBP_Player (Game|GetPlayerCharacter 0)))
      (Variables|Default|SetPlayerRef _asbp_player))))

(fn Destroy
  (Actor|DestroyActor))