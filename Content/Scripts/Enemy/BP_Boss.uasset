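; BP_Boss is an enemy boss Blueprint that counts its death toward the game's win condition.
; On BeginPlay it runs the parent logic, then casts the game mode to BP_GameplayGM and caches it.
; EventDead increments the game mode's CurrentBossesDead counter and calls CheckWinGame.
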(event EventBeginPlay
  (|CallParentFunction)
  (bind _asbp_gameplay_gm (Utilities|Casting|CastToBP_GameplayGM (Game|GetGameMode)))
  (Variables|Default|SetAs%20BP%20Gameplay%20GM _asbp_gameplay_gm))

(event Collision|EventActorBeginOverlap
  (params (OtherActor :type Actor%20Object%20Reference)))

(event EventTick
  (params (DeltaSeconds :type Float%20%28single-precision%29))
  (|CallParentFunction DeltaSeconds) ; This node is disabled and will not be called.\nDrag off pins to build functionality.
)

(event EventEventDead
  (bind _as_bp_gameplay_gm (Variables|Default|GetAs%20BP%20Gameplay%20GM))
  (Math|Integer|IncrementInt (Variables|/Game/Scripts/GameMode/BP_GameplayGM.BP_GameplayGM_C|GetcurrentBossesDead _as_bp_gameplay_gm)
    (:%20%20
      (Default|CheckWinGame _as_bp_gameplay_gm))))

(fn ConstructionScript
  (|CallParentFunction))