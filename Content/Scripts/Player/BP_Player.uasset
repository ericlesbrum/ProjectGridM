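; Player Character that handles movement, look, firing, interaction, pausing, health and death.
; It spawns a socket-attached BP_Gun, forwarding fire input to its trigger and UI and pause calls to BP_PlayerController.
; A camera sphere trace uses interfaces to collect colored keys, announced through dispatchers, or trigger interactive actors.
; Damage starts a looping, DoOnce-guarded regen timer that stops at full health or on death, which also broadcasts PlayerDead.
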(event Custom|Dead
  (Utilities|FlowControl|DoOnce false
    (:Completed
      (Utilities|Time|ClearTimerbyFunctionName 0 "RestoreHealth")
      (Default|UpdateUI (Variables|Default|GetBPPlayerController))
      (Variables|Default|SetisDead true)
      (Default|CallPlayerDead)
      (Default|DesactiveTrigger (Variables|Default|GetGun))
      (Variables|Default|SetisFiring false))))

(event Custom|DamageTaken
  (params (damage :type Integer))
  (Utilities|FlowControl|Sequence
    (:then_0
      (bind _output_get (Variables|Default|Sethealth (- (Variables|Default|Gethealth) damage)))
      (if (<= _output_get 0)
        (CallFunction|Dead)
        (else
          (Default|UpdateUI (Variables|Default|GetBPPlayerController)))))
    (:then_1
      (Utilities|FlowControl|DoOnce false
        (:Completed
          (Utilities|Time|SetTimerbyFunctionName 0 "RestoreHealth" 2.0 true))))))

(event Custom|ResetRegen
  (Utilities|FlowControl|DoOnce false) ; enters at Reset
)

(event Custom|PlayerRestartDeadState
  (Utilities|FlowControl|DoOnce false) ; enters at Reset
)

(event EventBeginPlay
  (bind _skeletalmesh (Variables|Default|GetSkeletalMesh))
  (Utilities|FlowControl|Sequence
    (:then_0
      (bind _returnvalue (Game|SpawnActorfromClass "/Game/Scripts/Gun/BP_Gun.BP_Gun_C" (Transformation|GetWorldTransform _skeletalmesh) "Undefined" "MultiplyWithRoot" 0 0))
      (Variables|Default|SetGun _returnvalue)
      (Transformation|AttachComponentToComponent _returnvalue _skeletalmesh "GunSocket" "SnapToTarget" "SnapToTarget" "SnapToTarget" true))
    (:then_1
      (bind _asbp_player_controller (Utilities|Casting|CastToBP_PlayerController (Game|GetPlayerController 0)))
      (Variables|Default|SetBPPlayerController _asbp_player_controller))
    (:then_2
      (Default|UpdateUI (Variables|Default|GetBPPlayerController)))))

(event Collision|EventActorBeginOverlap
  (params (OtherActor :type Actor%20Object%20Reference)))

(event EventTick
  (params (DeltaSeconds :type Float%20%28single-precision%29)))

(event Input|ActionEvents|InputActionJumpButton
  (params (Key :type Key%20Structure :default "None"))
  ;[1 1 1] Movimentação Básica
  (:Pressed
    (Character|Jump))
  (:Released
    (Character|StopJumping)))

(event Input|ActionEvents|InputActionRunning
  (params (Key :type Key%20Structure :default "None"))
  (bind _charactermovement (Variables|Character|GetCharacterMovement))
  ;[1 1 1] Movimentação Básica
  (:Pressed
    (Variables|/Script/Engine.CharacterMovementComponent|SetMaxWalkSpeed _charactermovement (Variables|Default|GetrunSpeed)))
  (:Released
    (Variables|/Script/Engine.CharacterMovementComponent|SetMaxWalkSpeed _charactermovement (Variables|Default|GetwalkSpeed))))

(event Input|ActionEvents|InputActionCrouching
  (params (Key :type Key%20Structure :default "None"))
  ;[1 1 1] Movimentação Básica
  (:Pressed
    (Character|Crouch))
  (:Released
    (Character|UnCrouch)))

(event Input|ActionEvents|InputActionFireButton
  (params (Key :type Key%20Structure :default "None"))
  (bind _gun (Variables|Default|GetGun))
  ;[1 1 1] Movimentação Básica
  (:Pressed
    (Variables|Default|SetisFiring true)
    (Default|ActiveTrigger _gun))
  (:Released
    (Variables|Default|SetisFiring false)
    (Default|DesactiveTrigger _gun)))

(event Input|ActionEvents|InputActionPauseButton
  (params (Key :type Key%20Structure :default "None"))
  (bind _bpplayercontroller (Variables|Default|GetBPPlayerController))
  (:Pressed
    (if (Game|IsGamePaused)
      (Default|UnPauseGame _bpplayercontroller)
      (else
        (Default|PauseGame _bpplayercontroller)))))

(event Input|ActionEvents|InputActionInteractButton
  (params (Key :type Key%20Structure :default "None"))
  (bind _camera (Variables|Default|GetCamera))
  (bind _returnvalue (Transformation|GetWorldLocation _camera))
  (:Pressed
    (bind _outhit (Collision|SphereTraceByChannel _returnvalue (+ _returnvalue (* (Math|Vector|GetForwardVector _camera) 3e+02)) 1e+02 "TraceTypeQuery1" false 0 "None"))
    (if (Utilities|DoesObjectImplementInterface (.HitActor (Collision|BreakHitResult _outhit)) "/Game/Scripts/Key/IBP_Pickup.IBP_Pickup_C")
      (bind _key (Class|IBPPickup|Pickup(Message) (.HitActor (Collision|BreakHitResult _outhit))))
      (switch Utilities|FlowControl|Switch|SwitchonEBP_Keys _key
        (:NewEnumerator0
          (Default|CallPickKeyGreen))
        (:NewEnumerator1
          (Default|CallPickKeyPink))
        (:NewEnumerator2
          (Default|CallPickKeyBlue)))
      (Actor|DestroyActor (.HitActor (Collision|BreakHitResult _outhit)))
      (elif (Utilities|DoesObjectImplementInterface (.HitActor (Collision|BreakHitResult _outhit)) "/Game/Scripts/Totem/IBP_Interactive.IBP_Interactive_C")
        (Class|IBPInteractive|Interact(Message) (.HitActor (Collision|BreakHitResult _outhit)))))))

(event Input|AxisEvents|InputAxisHorizontal
  (params (AxisValue :type Float%20%28single-precision%29))
  ;[1 1 1] Movimentação Básica
  (Pawn|Input|AddMovementInput (Math|Vector|GetRightVector (Variables|Collision|GetCapsuleComponent)) AxisValue false))

(event Input|AxisEvents|InputAxisVertical
  (params (AxisValue :type Float%20%28single-precision%29))
  ;[1 1 1] Movimentação Básica
  (Pawn|Input|AddMovementInput (Math|Vector|GetForwardVector (Variables|Collision|GetCapsuleComponent)) AxisValue false))

(event Input|AxisEvents|InputAxisMouseXInput
  (params (AxisValue :type Float%20%28single-precision%29))
  ;[1 1 1] Movimentação Básica
  (Pawn|Input|AddControllerYawInput AxisValue))

(event Input|AxisEvents|InputAxisMouseYInput
  (params (AxisValue :type Float%20%28single-precision%29))
  ;[1 1 1] Movimentação Básica
  (Pawn|Input|AddControllerPitchInput AxisValue))

(fn ConstructionScript)

(fn RestoreHealth
  (if (>= (+ (Variables|Default|Gethealth) 10) 100)
    (Variables|Default|Sethealth 100)
    (Utilities|Time|ClearTimerbyFunctionName 0 "RestoreHealth")
    (CallFunction|ResetRegen)
    (else
      (Variables|Default|Sethealth (+ (Variables|Default|Gethealth) 10))))
  (Default|UpdateUI (Variables|Default|GetBPPlayerController)))