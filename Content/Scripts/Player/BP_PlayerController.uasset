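; Player controller that owns the player's UI: HUD, pause menu and death menu.
; On BeginPlay it caches the BP_Player character, creates all three widgets and shows only the HUD.
; UpdateUI copies player health to the HUD text and progress bar, assuming a maximum of 100.
; PauseGame and UnPauseGame toggle game pause, swap HUD and pause menu, and switch cursor and input mode; the death menu is never displayed here.
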(event Custom|UpdateUI
  (bind _as_bp_player (Variables|Default|GetAs%20BP%20Player))
  (bind _hud (Variables|Default|GetHUD))
  (bind _health (Variables|/Game/Scripts/Player/BP_Player.BP_Player_C|Gethealth _as_bp_player))
  (Variables|/Game/HUD/BP_HUD.BP_HUD_C|SethealthHud (Variables|Default|GetHUD) (Utilities|Text|ToText(Integer) _health))
  (if (<= _health 0)
    (Variables|/Game/HUD/BP_HUD.BP_HUD_C|SetProgressBar _hud 0.0)
    (else
      (Variables|/Game/HUD/BP_HUD.BP_HUD_C|SetProgressBar _hud (Math|Float|SafeDivide (Math|Conversions|ToFloat(Integer) _health) 1e+02)))))

(event Custom|PauseGame
  (bind _pausemenu (Variables|Default|GetPauseMenu))
  (Game|SetGamePaused true)
  (Widget|RemovefromParent (Variables|Default|GetHUD))
  (UserInterface|Viewport|AddtoViewport _pausemenu 0)
  (Variables|Default|SetbShowMouseCursor true)
  (Input|SetInputModeGameandUI self _pausemenu "DoNotLock" true false))

(event Custom|UnPauseGame
  (Game|SetGamePaused false)
  (Widget|RemovefromParent (Variables|Default|GetPauseMenu))
  (UserInterface|Viewport|AddtoViewport (Variables|Default|GetHUD) 0)
  (Variables|Default|SetbShowMouseCursor false)
  (Input|SetInputModeGameOnly self false))

(event EventBeginPlay
  (bind _self self)
  (Utilities|FlowControl|Sequence
    (:then_0
      (bind _asbp_player (Utilities|Casting|CastToBP_Player (Game|GetPlayerCharacter 0)))
      (Variables|Default|SetAs%20BP%20Player _asbp_player))
    (:then_1
      (bind _returnvalue (UserInterface|CreateWidget "/Game/HUD/BP_HUD.BP_HUD_C" _self))
      (bind _output_get (Variables|Default|SetHUD _returnvalue))
      (UserInterface|Viewport|AddtoViewport _output_get 0))
    (:then_2
      (bind _returnvalue_2 (UserInterface|CreateWidget "/Game/HUD/BP_PauseMenu.BP_PauseMenu_C" _self))
      (Variables|Default|SetPauseMenu _returnvalue_2))
    (:then_3
      (bind _returnvalue_3 (UserInterface|CreateWidget "/Game/HUD/BP_DeadMenu.BP_DeadMenu_C" _self))
      (Variables|Default|SetDeadMenu _returnvalue_3))))

(event EventTick
  (params (DeltaSeconds :type Float%20%28single-precision%29)))

(fn ConstructionScript)