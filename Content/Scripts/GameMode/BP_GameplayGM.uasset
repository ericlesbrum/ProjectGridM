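; Gameplay game mode that handles player death and respawn, key pickups and totem activation for the level.
; On death it hides the player, possesses the first checkpoint, stops enemies and shows the death menu, whose restart respawns the player there and resets health, UI and enemies.
; Player pickup events update three colored HUD keys and a counter.
; Once all totems report active, a dispatcher opens the boss level.
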(event Custom|PlayerDead_Event
  (CallFunction|HidePlayer)
  (CallFunction|PossesCheckpoint)
  (CallFunction|StopAllEnemies)
  (CallFunction|AddDeadMenuHideHUD)
  (EventDispatchers|AssignRestart (Variables|/Game/Scripts/Player/BP_PlayerController.BP_PlayerController_C|GetDeadMenu (Variables|Default|GetAs%20BP%20Player%20Controller)) (delegate Custom|Restart_Event)))

(event Custom|Restart_Event
  (CallFunction|PossesPlayer)
  (CallFunction|UnHidePlayer)
  (CallFunction|SetPlayerPosition)
  (CallFunction|RemoveDeadMenuAddHUD)
  (CallFunction|RestartPlayerStatus)
  (Default|UpdateUI (Variables|Default|GetAs%20BP%20Player%20Controller))
  (CallFunction|ResetAllEnemies))

(event Custom|PickKeyBlue_Event
  (Default|SetKeyBlue (Variables|/Game/Scripts/Player/BP_PlayerController.BP_PlayerController_C|GetHUD (Variables|Default|GetAs%20BP%20Player%20Controller)))
  (Variables|Default|SetpickUpBlue true)
  (CallFunction|IncrementKeys))

(event Custom|PickKeyGreen_Event
  (Default|SetKeyGreen (Variables|/Game/Scripts/Player/BP_PlayerController.BP_PlayerController_C|GetHUD (Variables|Default|GetAs%20BP%20Player%20Controller)))
  (Variables|Default|SetpickUpGreen true)
  (CallFunction|IncrementKeys))

(event Custom|PickKeyPink_Event
  (Default|SetKeyPink (Variables|/Game/Scripts/Player/BP_PlayerController.BP_PlayerController_C|GetHUD (Variables|Default|GetAs%20BP%20Player%20Controller)))
  (Variables|Default|SetpickUpPink true)
  (CallFunction|IncrementKeys))

(event Custom|AllTotemsActive_Event
  (Game|OpenLevel(byName) "02Boss"))

(event EventBeginPlay
  (Utilities|FlowControl|Sequence
    (:then_0
      (bind _asbp_player (Utilities|Casting|CastToBP_Player (Game|GetPlayerCharacter 0)))
      (Variables|Default|SetPlayer _asbp_player)
      (EventDispatchers|AssignPlayerDead (Variables|Default|GetPlayer) (delegate Custom|PlayerDead_Event)))
    (:then_1
      (bind _asbp_player_controller (Utilities|Casting|CastToBP_PlayerController (Game|GetPlayerController 0)))
      (Variables|Default|SetAs%20BP%20Player%20Controller _asbp_player_controller))
    (:then_2
      (EventDispatchers|AssignPickKeyGreen (Variables|Default|GetPlayer) (delegate Custom|PickKeyGreen_Event)))
    (:then_3
      (EventDispatchers|AssignPickKeyPink (Variables|Default|GetPlayer) (delegate Custom|PickKeyPink_Event)))
    (:then_4
      (EventDispatchers|AssignPickKeyBlue (Variables|Default|GetPlayer) (delegate Custom|PickKeyBlue_Event)))
    (:then_5
      (bind _outactors (Actor|GetAllActorsOfClass "/Game/Scripts/Totem/BP_Totem.BP_Totem_C"))
      (Variables|Default|SettotemLength (Utilities|Array|Length _outactors))
      (EventDispatchers|BindEventtoAllTotemsActive (delegate Custom|AllTotemsActive_Event)))))

(fn ConstructionScript)

(fn HidePlayer
  (bind _player (Variables|Default|GetPlayer))
  (Rendering|SetActorHiddenInGame _player true)
  (Rendering|SetActorHiddenInGame (Variables|/Game/Scripts/Player/BP_Player.BP_Player_C|GetGun _player) true))

(fn UnHidePlayer
  (bind _player (Variables|Default|GetPlayer))
  (Rendering|SetActorHiddenInGame _player false)
  (Rendering|SetActorHiddenInGame (Variables|/Game/Scripts/Player/BP_Player.BP_Player_C|GetGun _player) false))

(fn PossesCheckpoint
  (bind _outactors (Actor|GetAllActorsOfClass "/Game/Scripts/Player/BP_Checkpoint.BP_Checkpoint_C"))
  (Pawn|Possess (Game|GetPlayerController 0) (Utilities|Array|Get(acopy) _outactors)))

(fn StopAllEnemies
  (bind _outactors (Actor|GetAllActorsOfClass "/Game/Scripts/Enemy/BP_Enemy.BP_Enemy_C"))
  (for _array_element _outactors
    (Default|StopEnemy _array_element)))

(fn AddDeadMenuHideHUD
  (bind _as_bp_player_controller (Variables|Default|GetAs%20BP%20Player%20Controller))
  (bind _deadmenu (Variables|/Game/Scripts/Player/BP_PlayerController.BP_PlayerController_C|GetDeadMenu _as_bp_player_controller))
  (Widget|RemovefromParent (Variables|/Game/Scripts/Player/BP_PlayerController.BP_PlayerController_C|GetHUD _as_bp_player_controller))
  (UserInterface|Viewport|AddtoViewport _deadmenu 0)
  (Input|SetInputModeUIOnly _as_bp_player_controller _deadmenu "DoNotLock" false)
  (Variables|/Script/Engine.PlayerController|SetbShowMouseCursor _as_bp_player_controller true))

(fn PossesPlayer
  (Pawn|Possess (Game|GetPlayerController 0) (Variables|Default|GetPlayer)))

(fn SetPlayerPosition
  (bind _player (Variables|Default|GetPlayer))
  (bind _outactors (Actor|GetAllActorsOfClass "/Game/Scripts/Player/BP_Checkpoint.BP_Checkpoint_C"))
  (Transformation|SetActorTransform _player (Transformation|GetActorTransform (Utilities|Array|Get(acopy) _outactors)))
  (Pawn|SetControlRotation (Pawn|GetController _player) (Transformation|GetActorRotation (Utilities|Array|Get(acopy) _outactors))))

(fn RemoveDeadMenuAddHUD
  (bind _as_bp_player_controller (Variables|Default|GetAs%20BP%20Player%20Controller))
  (Widget|RemovefromParent (Variables|/Game/Scripts/Player/BP_PlayerController.BP_PlayerController_C|GetDeadMenu _as_bp_player_controller))
  (UserInterface|Viewport|AddtoViewport (Variables|/Game/Scripts/Player/BP_PlayerController.BP_PlayerController_C|GetHUD _as_bp_player_controller) 0)
  (Input|SetInputModeGameOnly _as_bp_player_controller false)
  (Variables|/Script/Engine.PlayerController|SetbShowMouseCursor _as_bp_player_controller false))

(fn RestartPlayerStatus
  (bind _player (Variables|Default|GetPlayer))
  (Variables|/Game/Scripts/Player/BP_Player.BP_Player_C|Sethealth _player 100)
  (Variables|/Game/Scripts/Player/BP_Player.BP_Player_C|SetisDead _player false)
  (Default|PlayerRestartDeadState _player))

(fn ResetAllEnemies
  (bind _outactors (Actor|GetAllActorsOfClass "/Game/Scripts/Enemy/BP_Enemy.BP_Enemy_C"))
  (for _array_element _outactors
    (Default|RestartEnemy _array_element)
    (Default|ResetStatus _array_element)))

(fn IncrementKeys
  (bind _result (Math|Integer|IncrementInt (Variables|Default|GetkeyCount))
    (:%20%20
      (if (== _result 3)
        (Development|PrintString "Pode ir para porta final")))))

(fn CheckifAllTotemsActive
  (bind _result (Math|Integer|IncrementInt (Variables|Default|GetnumberOfTotemsActive))
    (:%20%20
      (if (== _result (Variables|Default|GettotemLength))
        (Default|CallAllTotemsActive)))))