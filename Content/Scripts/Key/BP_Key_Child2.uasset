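; BP_Key_Child2 is a key variant that gives its inherited key a pink glow color.
; Its construction script runs the parent's, then creates dynamic instances of M_keyglow on material slot 1 of Frame1 and Frame2 and sets their color parameter.
; The event graph holds only disabled placeholder nodes, so the child adds no event logic of its own.
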(event EventBeginPlay
  (|CallParentFunction) ; This node is disabled and will not be called.\nDrag off pins to build functionality.
)

(event Collision|EventActorBeginOverlap
  (params (OtherActor :type Actor%20Object%20Reference))
  (|CallParentFunction OtherActor) ; This node is disabled and will not be called.\nDrag off pins to build functionality.
)

(event EventTick
  (params (DeltaSeconds :type Float%20%28single-precision%29))
  (|CallParentFunction DeltaSeconds) ; This node is disabled and will not be called.\nDrag off pins to build functionality.
)

(fn ConstructionScript
  (|CallParentFunction)
  (bind _returnvalue (Rendering|Material|CreateDynamicMaterialInstance (Variables|Default|Getframe1) 1 "/Game/Models/Key/M_keyglow.M_keyglow" "None" :!class /Script/Engine.PrimitiveComponent))
  (Rendering|Material|SetVectorParameterValue _returnvalue "Param" "(R=1.000000,G=0.000000,B=0.575467,A=1.000000)" :!class /Script/Engine.MaterialInstanceDynamic)
  (bind _returnvalue_2 (Rendering|Material|CreateDynamicMaterialInstance (Variables|Default|Getframe2) 1 "/Game/Models/Key/M_keyglow.M_keyglow" "None" :!class /Script/Engine.PrimitiveComponent))
  (Rendering|Material|SetVectorParameterValue _returnvalue_2 "Param" "(R=1.000000,G=0.000000,B=0.576471,A=1.000000)" :!class /Script/Engine.MaterialInstanceDynamic))